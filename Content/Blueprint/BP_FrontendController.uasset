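; Frontend controller Blueprint that starts showcase background music and sets up UI, game settings and input for the frontend.
; BeginPlay plays the music as a 2D sound, while the end of the loading screen registers the plugin's default frontend UI config.
; On success, it runs and applies a hardware benchmark if no valid results exist, applies game settings, then registers a test mapping context with Enhanced Input user settings.
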(event `self.ReceiveBeginPlay`
  (bind _returnvalue (`GameplayStatics.CreateSound2D` "/CommonFrontendUI/Audio/MSS_BGM_Plugin_ShowCase.MSS_BGM_Plugin_ShowCase" 1.0 1.0 0.0 null))
  (`AudioComponent.Play` _returnvalue 0.0))

(event `CommonFrontendLoadingScreenInterface.OnLoadingScreenEnded`
  (`AsyncAction_RegisterFrontendUI_Config.RegisterFrontendUI_Config` "/CommonFrontendUI/CFUDC_Default_Plugin.CFUDC_Default_Plugin"
    (:`OnSuccess`
      (`|ExecutionSequence`
        (:`then_0`
          (bind _returnvalue (`GameUserSettings.GetGameUserSettings`))
          (`/Engine/EditorBlueprintResources/StandardMacros.IsValid` _returnvalue
            (:`Is Valid`
              (if (not (`CommonFrontendLibrary.HasValidBenchmarkSettings`))
                (`GameUserSettings.RunHardwareBenchmark` _returnvalue 10 1.0 1.0)
                (`GameUserSettings.ApplyHardwareBenchmarkResults` _returnvalue)))))
        (:`then_1`
          (bind _returnvalue_2 (`GameUserSettings.GetGameUserSettings`))
          (`/Engine/EditorBlueprintResources/StandardMacros.IsValid` _returnvalue_2
            (:`Is Valid`
              (`GameUserSettings.ApplySettings` _returnvalue_2 true))))
        (:`then_2`
          (`EnhancedInputUserSettings.RegisterInputMappingContext` (`EnhancedInputSubsystemInterface.GetUserSettings` (subsystem `EnhancedInputLocalPlayerSubsystem`)) "/CommonFrontendUI/Blueprint/Input/IMC_Test.IMC_Test"))))))

(fn `UserConstructionScript`)